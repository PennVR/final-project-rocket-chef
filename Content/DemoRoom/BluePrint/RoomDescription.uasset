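; Diner station actor that seats an arriving robot and takes fuel orders delivered by the player.
; An overlapping robot attaches to the stand and starts a one-second timer countdown shown with its order.
; A correct player delivery destroys the robot and frees the diner via OurGameState; a timeout updates the out-of-service count and starts flickering red spotlights.
; A timeline adds bobbing motion, and the construction script tints the stand through dynamic materials.
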(event `self.ReceiveActorBeginOverlap`
  (params (OtherActor :type "Actor Object Reference"))
  ;[1 1 1] Character Reached Diner with an order...
  (cast `/Game/FirstPersonBP/Blueprints/FirstPersonCharacter` OtherActor
    (:`then`
      (bind _asour_game_state (cast `/Game/FirstPersonBP/OurGameState` (`GameplayStatics.GetGameState`)))
      ;[1 1 1] Check if the player's current prepared order is the same as the one the robot at this dinner wants
      (bind _returnvalue (`RobotCharacter2.CheckRecipe` (`self.RobotRef`) (`/Game/FirstPersonBP/OurGameState.FuelTemp` _asour_game_state) (`/Game/FirstPersonBP/OurGameState.FuelColor` _asour_game_state) (`/Game/FirstPersonBP/OurGameState.FuelFlavor` _asour_game_state)))
      (if _returnvalue
        (`KismetSystemLibrary.PrintString` "Correct order delivered!")
        ;[1 1 1] ...if correct, reset the diner!
        (set `self.RobotAtDiner` false)
        (`/Game/FirstPersonBP/OurGameState.DinerReady` _asour_game_state (`/Game/FirstPersonBP/RobotCharacter2_Blueprint.DinerNumber` (`self.RobotRef`)))
        (`self.K2_DestroyActor` (`self.RobotRef`))
        (`TextRenderComponent.K2_SetText` (`self.DinerDisplay`) (`|FormatText` "Order Complete!"))
        (set `self.TimerCount` (`/Game/FirstPersonBP/OurGameState.DinerTimer` _asour_game_state))
        (else
          (`KismetSystemLibrary.PrintString` "Incorrect order!"))))
    (:`CastFailed`
      ;[1 1 1] Set Config Variables for when the robot initially spawns at a diner
      (bind _asrobot_character_2_blueprint (cast `/Game/FirstPersonBP/RobotCharacter2_Blueprint` OtherActor))
      (`self.K2_AttachToComponent` _asrobot_character_2_blueprint (`self.SM_Base`) "None" "SnapToTarget" "KeepRelative" "KeepRelative" false)
      (`RobotCharacter2.GetRecipe` _asrobot_character_2_blueprint)
      (set `self.RobotRef` _asrobot_character_2_blueprint)
      (set `self.Recipe` (`KismetMathLibrary.RandomIntegerInRange` 1 10))
      (set `self.RobotAtDiner` true)
      ;[1 1 1] Decrement the diner's timer while the robot is at the station
      (if (and (>= (`self.TimerCount`) 0) (`self.RobotAtDiner`)) :!label _label
        (`TextRenderComponent.K2_SetText` (`self.DinerDisplay`) (`KismetTextLibrary.Conv_StringToText` (`KismetStringLibrary.Concat_StrStr` (`|GetEnumeratorNameAsString` (`RobotCharacter2.FuelTempEnum` (`self.RobotRef`))) " " (`|GetEnumeratorNameAsString` (`RobotCharacter2.FuelColorEnum` (`self.RobotRef`))) " " (`|GetEnumeratorNameAsString` (`RobotCharacter2.FuelFlavorEnum` (`self.RobotRef`))) " " "Fuel" "    " (`KismetStringLibrary.Conv_IntToString` (`self.TimerCount`)))))
        (`KismetSystemLibrary.K2_SetTimerDelegate` (delegate `DecrementTimer`) 1.0)
        (else
          ;[1 1 1] Decrement the number of diners in comission globally
          (if (`self.RobotAtDiner`)
            (bind _asour_game_state_2 (cast `/Game/FirstPersonBP/OurGameState` (`GameplayStatics.GetGameState`)))
            (bind _result (`/Engine/EditorBlueprintResources/StandardMacros.DecrementInt` (`/Game/FirstPersonBP/OurGameState.NumberOfDinersOutOfService` _asour_game_state_2))
              (:`  `
                (set `/Game/FirstPersonBP/OurGameState.NumberOfDinersOutOfService` _result _asour_game_state_2)
                ;[1 1 1] Set the diner text and the light color/intensity
                (`TextRenderComponent.K2_SetText` (`self.DinerDisplay`) (`|FormatText` "Out of service"))
                (`LightComponent.SetLightColor` (`self.SpotLight`) (struct :`R` 255.0 :`A` 1.0) true)
                (`LightComponent.SetLightColor` (`self.SpotLight2`) (struct :`R` 255.0 :`A` 1.0) true)
                (`LightComponent.SetIntensity` (`self.SpotLight`) 200000.0)
                (`LightComponent.SetIntensity` (`self.SpotLight2`) 200000.0)
                ;[1 1 1] If the diner goes down, flicker the lights every 0.1 seconds
                (`KismetSystemLibrary.K2_SetTimerDelegate` (delegate `FlickerLight`) 0.1 true)))))))))

(event `DecrementTimer`
  ;[1 1 1] Decrement the diner's timer while the robot is at the station
  (bind _result (`/Engine/EditorBlueprintResources/StandardMacros.DecrementInt` (`self.TimerCount`))
    (:`  `
      (set `self.TimerCount` _result)
      (goto _label))))

(event `self.ReceiveTick`
  (params (DeltaSeconds :type "Float (single-precision)")))

(event `self.ReceiveBeginPlay`
  ;[1 1 1] Bob up and down!
  (`KismetSystemLibrary.K2_SetTimerDelegate` (delegate `CustomEvent_0`) (`KismetMathLibrary.RandomFloatInRange` 0.0 5.0))
  (set `self.OriginalLocation` (`self.K2_GetActorLocation`))
  (bind (_direction _newtrack_0) (`Timeline|Timeline_0` :!label _label_2)
    (:`Update`
      (`self.K2_SetActorRelativeLocation` (+ (`self.OriginalLocation`) _newtrack_0)))))

(event `CustomEvent_0`
  ;[1 1 1] Bob up and down!
  (goto _label_2 :!via `Reverse`))

(event `FlickerLight`
  ;[1 1 1] If the diner goes down, flicker the lights every 0.1 seconds
  (`SceneComponent.ToggleVisibility` (`self.SpotLight`) false)
  (`SceneComponent.ToggleVisibility` (`self.SpotLight2`) false))

(fn `UserConstructionScript`
  (bind _returnvalue (`PrimitiveComponent.CreateDynamicMaterialInstance` (`self.SM_Base`) 3 null))
  (`MaterialInstanceDynamic.SetVectorParameterValue` _returnvalue "Color" (`self.StandColor`))
  (bind _returnvalue_2 (`PrimitiveComponent.CreateDynamicMaterialInstance` (`self.SM_Base_FlatWall`) 0 null))
  (`MaterialInstanceDynamic.SetVectorParameterValue` _returnvalue_2 "Color" (`self.StandColor`)))